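; OLdmessi is an actor Blueprint that toggles an inspection-style view on Tab, with an object that the mouse can tumble.
; Tab flips IsPaused, switching the HUD and cursor and swapping visibility between Mesh and the Plane, Ew and Okok components, without actually pausing the game.
; While the left mouse button is held, Tick rotates Ew in world space from inverted input axis values scaled by TumbleSpeed, regardless of IsPaused.
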(event `Key|Tab`
  (params (Key :type "Key Structure"))
  (bind _returnvalue (`GameplayStatics.GetPlayerController` 0))
  (bind _plane (`self.Plane`))
  (bind _mesh (`self.Mesh`))
  (bind _returnvalue_2 (`PlayerController.GetHUD` _returnvalue))
  (:`Pressed`
    (if (`self.IsPaused`)
      (bind _output_get (set `HUD.bShowHUD` false _returnvalue_2))
      (set `PlayerController.bShowMouseCursor` _output_get _returnvalue)
      (set `self.IsPaused` false)
      (`SceneComponent.SetVisibility` _mesh true false)
      (`SceneComponent.SetVisibility` _plane false false)
      (`SceneComponent.SetVisibility` (`self.ew`) false false)
      (`SceneComponent.SetVisibility` (`self.okok`) false false)
      (else
        (bind _output_get_2 (set `HUD.bShowHUD` true _returnvalue_2))
        (set `PlayerController.bShowMouseCursor` _output_get_2 _returnvalue)
        (set `self.IsPaused` true)
        (`SceneComponent.SetVisibility` _plane true false)
        (`SceneComponent.SetVisibility` (`self.ew`) true false)
        (`SceneComponent.SetVisibility` (`self.okok`) true false)
        (`SceneComponent.SetVisibility` _mesh false false)))))

(event `Key|LeftMouseButton`
  (params (Key :type "Key Structure"))
  ;[1 1 1] Mouse
  (:`Pressed`
    (set `self.TumbleAction` true))
  (:`Released`
    (set `self.TumbleAction` false)))

(event `self.ReceiveTick`
  (params (DeltaSeconds :type "Float (single-precision)"))
  (bind _ew (`self.ew`))
  (bind _tumblespeed (`self.TumbleSpeed`))
  ;[1 1 1] Tumbler
  (if (`self.TumbleAction`)
    (`SceneComponent.K2_SetWorldRotation` _ew (`KismetMathLibrary.ComposeRotators` (`SceneComponent.K2_GetComponentRotation` _ew) (`KismetMathLibrary.MakeRotator` 0.0 (* (* (`self.GetInputAxisKeyValue`) -1.0) _tumblespeed) (* (* (`self.GetInputAxisKeyValue`) -1.0) _tumblespeed))) false false)))

(fn `UserConstructionScript`)