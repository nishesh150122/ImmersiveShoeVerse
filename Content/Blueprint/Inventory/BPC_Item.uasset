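; BPC_Item is an inventory component that records items and their prices for its owner.
; Separate add functions append to the item and price arrays, print the new entry, and forward it to the Inventory01 list on the owning BP_FirstPersonCharacter.
; CalculateTotalPrice converts each stored price to an integer and accumulates the sum.
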(fn `Add Item to Inventory`
  (params (NewItem :type "String (by ref)"))
  ;[1 1 1] Comment
  (`KismetArrayLibrary.Array_Add` (`self.inventory`) NewItem)
  (`KismetSystemLibrary.PrintString` NewItem)
  (bind _asbp_first_person_character (cast `/Game/FirstPerson/Blueprints/BP_FirstPersonCharacter` (`self.GetOwner`)))
  (`/Game/Blueprint/Inventory/WB_inventory01.Add item to List` (`/Game/FirstPerson/Blueprints/BP_FirstPersonCharacter.Inventory01` _asbp_first_person_character) NewItem))

(fn `CalculateTotalPrice`
  (returns (NewParam :type Integer))
  (for _array_element (`self.price001`)
    (bind _output_get (set `self.NewVar0` (+ (`KismetStringLibrary.Conv_StringToInt` _array_element) (`self.NewVar0`)))))
  (return _output_get))

(fn `Price Add 001`
  (params (NewItem :type "String (by ref)"))
  (`KismetArrayLibrary.Array_Add` (`self.price001`) NewItem)
  (`KismetSystemLibrary.PrintString` NewItem)
  (bind _asbp_first_person_character (cast `/Game/FirstPerson/Blueprints/BP_FirstPersonCharacter` (`self.GetOwner`)))
  (`/Game/Blueprint/Inventory/WB_inventory01.Add price to list` (`/Game/FirstPerson/Blueprints/BP_FirstPersonCharacter.Inventory01` _asbp_first_person_character) NewItem))